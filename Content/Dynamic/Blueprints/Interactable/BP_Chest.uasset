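; BP_Chest is a one-time interactable chest that swings its lid open and spawns a configured actor.
; It extends an interactable parent, registering the lid mesh for highlighting at BeginPlay.
; The first interaction destroys the detection component and plays a timeline rotating the lid pivot from its initial rotation.
; When the timeline finishes, the actor spawns at a marker point with a confetti effect and party horn sound.
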(event EventBeginPlay
  (|CallParentFunction)
  (Variables|Utility|SetinitialTopRotation (Variables|/Script/Engine.SceneComponent|GetRelativeRotation (Variables|Default|GetTopPivot)))
  (Utilities|Array|Add (Variables|Default|GethighlightedMeshes) (Variables|Default|GetTop)))

(event Collision|EventActorBeginOverlap
  (params (OtherActor :type Actor%20Object%20Reference))
  (|CallParentFunction OtherActor) ; This node is disabled and will not be called.\nDrag off pins to build functionality.
)

(event EventTick
  (params (DeltaSeconds :type Float%20%28single-precision%29))
  (|CallParentFunction DeltaSeconds) ; This node is disabled and will not be called.\nDrag off pins to build functionality.
)

(event EventInteract
  (params (interactor :type Actor%20Object%20Reference))
  (bind _spawnedopbjectpoint (Variables|Default|GetSpawnedOpbjectPoint))
  (bind _returnvalue (Transformation|GetWorldLocation _spawnedopbjectpoint))
  (|CallParentFunction interactor)
  (if (not (Variables|Utility|GetalreadyOpened))
    (Components|DestroyComponent (Variables|Default|GetInteractionDetection))
    (Variables|Utility|SetalreadyOpened true)
    (bind _alpha (Timeline|AnimateChest PlayFromStart)
      (:Update
        (Transformation|SetRelativeRotation (Variables|Default|GetTopPivot) (Math|Rotator|Lerp(Rotator) (Variables|Utility|GetinitialTopRotation) (Math|Rotator|CombineRotators "0, 0, 0" (Math|Rotator|MakeRotator -45.0 0.0 0.0)) _alpha true) false false))
      (:Finished
        (Game|SpawnActorfromClass (Variables|References|GetinteractableToSpawn) (Transformation|GetWorldTransform (Variables|Default|GetSpawnedOpbjectPoint)) "Undefined" 0 0)
        (Effects|SpawnEmitteratLocation "/Game/Static/Art/Particles/PS_Conffeti.PS_Conffeti" _returnvalue "0, 0, 0" "1.000000,1.000000,1.000000" true "AutoRelease")
        (Audio|PlaySoundatLocation "/Game/Static/Audio/SFX/Party-Horn-Sound-Effect.Party-Horn-Sound-Effect" _returnvalue "0, 0, 0" 1.0 1.0 0.0 0 0 0)))))

(fn ConstructionScript
  (|CallParentFunction))