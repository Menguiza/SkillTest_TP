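; BP_Door is an interactable door that swings 90 degrees in yaw to open or close and can be locked behind an inventory item.
; Interact checks the interactor through BI_InventoryOwner, consumes the required item to unlock, then toggles a timeline lerping from the initial rotation, guarded by IsMoving.
; First targeting and unlocking set custom depth stencil on highlighted meshes to show lock state.
; The ToogleDoor function is an empty stub.
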(event EventBeginPlay
  (|CallParentFunction)
  (Variables|Utility|SetinitialRotation (Transformation|GetActorRotation)))

(event Collision|EventActorBeginOverlap
  (params (OtherActor :type Actor%20Object%20Reference))
  (|CallParentFunction OtherActor) ; This node is disabled and will not be called.\nDrag off pins to build functionality.
)

(event EventTick
  (params (DeltaSeconds :type Float%20%28single-precision%29))
  (|CallParentFunction DeltaSeconds) ; This node is disabled and will not be called.\nDrag off pins to build functionality.
)

(event EventInteract
  (params (interactor :type Actor%20Object%20Reference))
  (bind _initialrotation (Variables|Utility|GetinitialRotation))
  (bind _openrequirement (Variables|References|GetopenRequirement))
  (|CallParentFunction interactor)
  (if (Variables|Parameters|GetisLocked)
    (bind _asbi_inventory_owner (Utilities|Casting|CastToBI_InventoryOwner interactor))
    (bind _result (Default|HasItem _asbi_inventory_owner _openrequirement))
    (if (and _result (not (Variables|Utility|GetisMoving)))
      (Default|ConsumeItem _asbi_inventory_owner _openrequirement)
      (Utilities|FlowControl|Sequence
        (:then_0
          (Variables|Parameters|SetisLocked false)
          (if (not (Variables|Utility|GetisMoving)) :!label _label
            (Variables|Utility|SetisMoving true)
            (if (Variables|Utility|GetisOpen)
              (bind _alpha (Timeline|DoorAnimation ReverseFromEnd)
                (:Update
                  (Transformation|SetActorRotation (Math|Rotator|Lerp(Rotator) _initialrotation (Math|Rotator|CombineRotators _initialrotation (Math|Rotator|MakeRotator 0.0 0.0 9e+01)) _alpha true)))
                (:Finished
                  (Variables|Utility|SetisOpen (not (Math|Rotator|Equal(Rotator) (Transformation|GetActorRotation) (Variables|Utility|GetinitialRotation) 0.0001)))
                  (Variables|Utility|SetisMoving false)))
              (else
                (Timeline|DoorAnimation PlayFromStart)))))
        (:then_1
          (for _array_element (Variables|Default|GethighlightedMeshes)
            (Utilities|IsValid _array_element
              (:Is%20Valid
                (Rendering|SetCustomDepthStencilValue _array_element (select (Variables|Parameters|GetisLocked) 3 2))))))))
    (else
      (goto _label))))

(event EventTargeted
  (if (not (Variables|Default|GetalreadyTargeted))
    (Variables|Default|SetalreadyTargeted true)
    (for _array_element (Variables|Default|GethighlightedMeshes)
      (Utilities|IsValid _array_element
        (:Is%20Valid
          (Rendering|SetCustomDepthStencilValue _array_element (select (Variables|Parameters|GetisLocked) 3 2)))))))

(fn ConstructionScript
  (|CallParentFunction))

(fn ToogleDoor
  (params (open :type Boolean))
  (if open
    _))