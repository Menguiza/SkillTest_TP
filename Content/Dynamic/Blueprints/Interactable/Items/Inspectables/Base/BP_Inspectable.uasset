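; Base Blueprint for inspectable items that an inspector can examine when interacting with them.
; On Interact it runs the parent logic, then continues only if the interactor implements the BI_Inspector interface.
; Its Inspect event passes the item's static mesh with initial inspection rotation and scale to the inspector's InitInspect, leaving the inspection itself to that inspector.
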(event EventBeginPlay
  (|CallParentFunction) ; This node is disabled and will not be called.\nDrag off pins to build functionality.
)

(event Collision|EventActorBeginOverlap
  (params (OtherActor :type Actor%20Object%20Reference))
  (|CallParentFunction OtherActor) ; This node is disabled and will not be called.\nDrag off pins to build functionality.
)

(event EventTick
  (params (DeltaSeconds :type Float%20%28single-precision%29))
  (|CallParentFunction DeltaSeconds))

(event EventInspect
  (params (inspector :type BI%20Inspector%20Interface))
  (Default|InitInspect inspector (Utilities|Struct|MakeS_InspectStruct (Variables|/Script/Engine.StaticMeshComponent|GetStaticMesh (Variables|Default|GetStaticMesh)) (Variables|Parameters|GetinspectInitalRotation) (Variables|Parameters|GetinspectInitialScale))))

(event EventInteract
  (params (interactor :type Actor%20Object%20Reference))
  (|CallParentFunction interactor)
  (bind _asbi_inspector (Utilities|Casting|CastToBI_Inspector interactor))
  (CallFunction|Inspect _asbi_inspector))

(fn ConstructionScript
  (|CallParentFunction))