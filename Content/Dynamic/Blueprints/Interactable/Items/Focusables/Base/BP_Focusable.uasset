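; Base interactable actor that lets a character focus on it, passing itself as view actor to the BI_Inspector interface with a blend time.
; Interact casts and stores the character and inspector, then Focus enables input on the actor, sets Game and UI mode, fades AffectedMeshes through an Opacity material parameter and disables InteractionDetection collision.
; Pressing the Interact input calls RequestFocus again and restores game-only input, opacity and query collision.
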(event EventBeginPlay
  (|CallParentFunction) ; This node is disabled and will not be called.\nDrag off pins to build functionality.
)

(event Collision|EventActorBeginOverlap
  (params (OtherActor :type Actor%20Object%20Reference))
  (|CallParentFunction OtherActor) ; This node is disabled and will not be called.\nDrag off pins to build functionality.
)

(event EventTick
  (params (DeltaSeconds :type Float%20%28single-precision%29))
  (|CallParentFunction DeltaSeconds) ; This node is disabled and will not be called.\nDrag off pins to build functionality.
)

(event EventInteract
  (params (interactor :type Actor%20Object%20Reference))
  (|CallParentFunction interactor)
  (bind _ascharacter (Utilities|Casting|CastToCharacter interactor))
  (bind _output_get (Variables|Utility|Setcharacter _ascharacter))
  (bind _asbi_inspector (Utilities|Casting|CastToBI_Inspector _output_get))
  (bind _output_get_2 (Variables|Utility|Setinspector _asbi_inspector))
  (CallFunction|Focus _output_get_2))

(event EventFocus
  (params (inspector :type BI%20Inspector%20Interface))
  (bind _character (Variables|Utility|Getcharacter))
  (bind _returnvalue (Pawn|GetController _character))
  (bind _asplayer_controller (Utilities|Casting|CastToPlayerController _returnvalue))
  (Default|RequestFocus inspector self (Variables|Parameters|GetblendTime))
  (Input|EnableInput _asplayer_controller)
  (Input|SetInputModeGameandUI _asplayer_controller 0 "LockAlways" false)
  (for _array_element (Variables|References|GetaffectedMeshes)
    (Rendering|Material|SetScalarParameterValueonMaterials (Variables|/Script/Engine.StaticMeshActor|GetStaticMeshComponent _array_element) "Opacity" 0.5))
  (Collision|SetCollisionEnabled (Variables|Default|GetInteractionDetection) "NoCollision"))

(event Input|ActionEvents|InputActionInteract
  (params (Key :type Key%20Structure :default "None"))
  (bind _character (Variables|Utility|Getcharacter))
  (bind _returnvalue (Pawn|GetController _character))
  (bind _asplayer_controller (Utilities|Casting|CastToPlayerController _returnvalue))
  (:Pressed
    (Default|RequestFocus (Variables|Utility|Getinspector) self (Variables|Parameters|GetblendTime))
    (Input|DisableInput _asplayer_controller)
    (Input|SetInputModeGameOnly _asplayer_controller)
    (for _array_element (Variables|References|GetaffectedMeshes)
      (Rendering|Material|SetScalarParameterValueonMaterials (Variables|/Script/Engine.StaticMeshActor|GetStaticMeshComponent _array_element) "Opacity" 1.0))
    (Collision|SetCollisionEnabled (Variables|Default|GetInteractionDetection) "QueryOnly")))

(fn ConstructionScript
  (|CallParentFunction))