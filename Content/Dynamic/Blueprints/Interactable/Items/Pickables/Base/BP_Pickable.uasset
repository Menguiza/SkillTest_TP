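; BP_Pickable is a base item actor that an interactor can pick up into an inventory.
; Interact calls the parent implementation, then casts the interactor to BI_InventoryOwner and stops if the cast fails.
; On success, Pick adds the pickable's ItemData to that inventory owner and destroys the actor.
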(event EventBeginPlay
  (|CallParentFunction) ; This node is disabled and will not be called.\nDrag off pins to build functionality.
)

(event Collision|EventActorBeginOverlap
  (params (OtherActor :type Actor%20Object%20Reference))
  (|CallParentFunction OtherActor) ; This node is disabled and will not be called.\nDrag off pins to build functionality.
)

(event EventTick
  (params (DeltaSeconds :type Float%20%28single-precision%29))
  (|CallParentFunction DeltaSeconds) ; This node is disabled and will not be called.\nDrag off pins to build functionality.
)

(event EventInteract
  (params (interactor :type Actor%20Object%20Reference))
  (|CallParentFunction interactor)
  (bind _asbi_inventory_owner (Utilities|Casting|CastToBI_InventoryOwner interactor))
  (CallFunction|Pick _asbi_inventory_owner))

(event EventPick
  (params (inventoryOwner :type BI%20Inventory%20Owner%20Interface))
  (Default|AddItem inventoryOwner (Variables|Default|GetitemData))
  (Actor|DestroyActor self))

(fn ConstructionScript
  (|CallParentFunction))