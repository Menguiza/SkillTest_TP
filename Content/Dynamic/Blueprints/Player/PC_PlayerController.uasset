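; Player controller that forwards movement and look input axes to a bound C_Player character.
; BindCharacter caches the character in MyPlayer after a cast, and UnBindCharacter clears it if it matches.
; Axis events check MyPlayer is valid, then add movement input along the controller's own forward and right vectors, or yaw and pitch input for the camera.
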(event EventBeginPlay)

(event EventTick
  (params (DeltaSeconds :type Float%20%28single-precision%29)))

(event Input|AxisEvents|InputAxisMoveForward
  (params (AxisValue :type Float%20%28single-precision%29))
  (bind __myplayer (Variables|Default|Get_myPlayer))
  ;[1 1 1] Movement
  (Utilities|IsValid __myplayer
    (:Is%20Valid
      (Pawn|Input|AddMovementInput __myplayer (Transformation|GetActorForwardVector) AxisValue false))))

(event Input|AxisEvents|InputAxisMoveRight
  (params (AxisValue :type Float%20%28single-precision%29))
  (bind __myplayer (Variables|Default|Get_myPlayer))
  ;[1 1 1] Movement
  (Utilities|IsValid __myplayer
    (:Is%20Valid
      (Pawn|Input|AddMovementInput __myplayer (Transformation|GetActorRightVector) AxisValue false))))

(event Input|AxisEvents|InputAxisTurn
  (params (AxisValue :type Float%20%28single-precision%29))
  (bind __myplayer (Variables|Default|Get_myPlayer))
  ;[1 1 1] Camera
  (Utilities|IsValid __myplayer
    (:Is%20Valid
      (Pawn|Input|AddControllerYawInput __myplayer AxisValue))))

(event Input|AxisEvents|InputAxisLookUp
  (params (AxisValue :type Float%20%28single-precision%29))
  (bind __myplayer (Variables|Default|Get_myPlayer))
  ;[1 1 1] Camera
  (Utilities|IsValid __myplayer
    (:Is%20Valid
      (Pawn|Input|AddControllerPitchInput __myplayer AxisValue))))

(fn ConstructionScript)

(fn BindCharacter
  (params (PossessedChar :type Character%20Object%20Reference))
  (bind _asc_player (Utilities|Casting|CastToC_Player PossessedChar))
  (Variables|Default|Set_myPlayer _asc_player))

(fn UnBindCharacter
  (params (UnpossessedChar :type Character%20Object%20Reference))
  (if (== UnpossessedChar (Variables|Default|Get_myPlayer))
    (Variables|Default|Set_myPlayer 0)))