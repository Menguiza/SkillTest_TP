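; Player inventory component that stores stackable items, creates its UI widget on BeginPlay and handles adding, consuming and dropping items.
; Parallel maps keyed by ItemData track quantities and BP_ItemObject wrappers, which update on quantity changes and are passed to WB_Inventory on add or removal.
; MaxItems caps distinct entries rather than stack size.
; DropItem consumes one of the first key's item, spawning its actor at SpawnPoint with a forward impulse.
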(event EventBeginPlay
  (bind _returnvalue (UserInterface|CreateWidget "/Game/Dynamic/Widgets/Inventory/WB_Inventory.WB_Inventory_C"))
  (UserInterface|Viewport|AddtoViewport _returnvalue 0)
  (Variables|Utility|SetinventoryWidget _returnvalue))

(event EventTick
  (params (DeltaSeconds :type Float%20%28single-precision%29)))

(fn AddItem
  (params (itemData :type PDA%20Inventory%20Item%20Asset%20Object%20Reference) (quantity :type Integer))
  (bind _inventory (Variables|Utility|Getinventory))
  (bind _inventorywidget (Variables|Utility|GetinventoryWidget))
  (bind _objectinventory (Variables|Utility|GetobjectInventory))
  (bind (_value _returnvalue) (Utilities|Map|Find _inventory itemData))
  (bind (_value_2 _returnvalue_2) (Utilities|Map|Find _objectinventory itemData))
  (bind _returnvalue_3 (+ _value quantity))
  (bind _returnvalue_4 (select _returnvalue _returnvalue_3 quantity))
  (if (and (select _returnvalue true (> (Variables|Parameters|GetMaxItems) (Utilities|Map|Length (Variables|Utility|Getinventory)))) (> quantity 0))
    (Utilities|FlowControl|Sequence
      (:then_0
        (if _returnvalue
          (if _returnvalue_2
            (Default|UpdateQuantity _value_2 _returnvalue_4))
          (else
            (bind _returnvalue_5 (Game|ConstructObjectfromClass "/Game/Dynamic/Blueprints/Items/BP_ItemObject.BP_ItemObject_C" self itemData _returnvalue_4))
            (Utilities|Map|Add (Variables|Utility|GetobjectInventory) itemData _returnvalue_5)
            (Utilities|IsValid _inventorywidget
              (:Is%20Valid
                (Default|ItemAdded _inventorywidget _returnvalue_5))))))
      (:then_1
        (Utilities|Map|Add (Variables|Utility|Getinventory) itemData _returnvalue_4)))))

(fn ConsumeItem
  (params (itemData :type PDA%20Inventory%20Item%20Asset%20Object%20Reference) (quantity :type Integer))
  (bind _inventory (Variables|Utility|Getinventory))
  (bind _inventorywidget (Variables|Utility|GetinventoryWidget))
  (bind _objectinventory (Variables|Utility|GetobjectInventory))
  (bind _inventory_2 (Variables|Utility|Getinventory))
  (bind (_value _returnvalue) (Utilities|Map|Find _inventory itemData))
  (bind (_value_2 _returnvalue_2) (Utilities|Map|Find _objectinventory itemData))
  (bind _returnvalue_3 (- _value quantity))
  (if (and _returnvalue (> quantity 0))
    (if (<= _returnvalue_3 0)
      (Utilities|Map|Remove _inventory_2 itemData)
      (Utilities|IsValid _inventorywidget
        (:Is%20Valid
          (Default|ItemRemoved _inventorywidget _value_2))
        (:Is%20Not%20Valid
          _))
      (Utilities|Map|Remove (Variables|Utility|GetobjectInventory) itemData)
      (else
        (Utilities|Map|Add _inventory_2 itemData _returnvalue_3)
        (if _returnvalue_2
          (Default|UpdateQuantity _value_2 (.Value (Utilities|Map|Find (Variables|Utility|Getinventory) itemData))))))))

(fn HasItem
  (params (item :type PDA%20Inventory%20Item%20Asset%20Object%20Reference))
  (return (Utilities|Map|Contains (Variables|Utility|Getinventory) item)))

(fn DropItem
  (bind _spawnpoint (Variables|References|GetspawnPoint))
  (Utilities|IsValid (Variables|References|GetspawnPoint)
    (:Is%20Valid
      (bind _keys (Utilities|Map|Keys (Variables|Utility|GetobjectInventory)))
      (bind _output_get (LocalVariables|SetitemSelected (Utilities|Array|Get(acopy) _keys)))
      (if (Utility|HasItem _output_get)
        (Behvaiors|ConsumeItem (LocalVariables|GetitemSelected) 1)
        (bind _returnvalue (Game|SpawnActorfromClass (Variables|/Game/Static/DataAssets/Items/Base/PDA_InventoryItemAsset.PDA_InventoryItemAsset_C|GetItemObject (LocalVariables|GetitemSelected)) (Transformation|GetWorldTransform _spawnpoint) "Undefined" 0 0))
        (Physics|AddImpulse (Variables|/Game/Dynamic/Blueprints/Interactable/Base/BP_Interactable.BP_Interactable_C|GetStaticMesh _returnvalue) (* (Math|Vector|GetForwardVector _spawnpoint) (* (Variables|Parameters|GetdropForce) 1e+02)) "None" false)))))

(fn SetSpawnPoint
  (params (spawnPoint :type Scene%20Component%20Object%20Reference))
  (Variables|References|SetspawnPoint spawnPoint))